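; Target spawner that places BP_Target actors at random points inside a box sized in the construction script.
; It binds to the first-person character's start and spawn dispatchers, spawning three targets on start and one per spawn call.
; Candidates near any of three remembered X positions are shifted randomly along X and rechecked.
; After each spawn and a one-tick delay, nested FlipFlops choose which remembered position to overwrite.
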(event `Start`
  (for _ (range 3)
    (`self.Spawn Target`)))

(event `self.ReceiveBeginPlay`
  (bind _asbp_first_person_character (cast `/Game/FirstPerson/Blueprints/BP_FirstPersonCharacter` (`GameplayStatics.GetPlayerCharacter` 0)))
  (bind _output_get (set `self.As BP First Person Character` _asbp_first_person_character))
  (add `/Game/FirstPerson/Blueprints/BP_FirstPersonCharacter.SpawnDispatch` _output_get (delegate `Spawn Target`))
  (add `/Game/FirstPerson/Blueprints/BP_FirstPersonCharacter.StartDispatch` (`self.As BP First Person Character`) (delegate `Start`)))

(event `Spawn Target`
  (bind _returnvalue (`KismetMathLibrary.RandomFloatInRange` 200.0 400.0))
  (bind (_newlocation_x _newlocation_y _newlocation_z) (`KismetMathLibrary.BreakVector` (`self.newLocation`)))
  (bind (_newlocation_x_2 _newlocation_y_2 _newlocation_z_2) (`KismetMathLibrary.BreakVector` (`self.newLocation`)))
  (bind _box (`self.Box`))
  (bind _newlocation (`self.newLocation`))
  (set `self.newLocation` (`KismetMathLibrary.RandomPointInBoundingBox` (`SceneComponent.K2_GetComponentLocation` _box) (`BoxComponent.GetScaledBoxExtent` _box)))
  (if (`self.IsCloseToAny?`) :!label _label
    (if (`KismetMathLibrary.RandomBool`)
      (set `self.newLocation` (`KismetMathLibrary.MakeVector` (- _newlocation_x _returnvalue) _newlocation_y _newlocation_z))
      (else
        (set `self.newLocation` (`KismetMathLibrary.MakeVector` (+ _newlocation_x_2 _returnvalue) _newlocation_y_2 _newlocation_z_2)))))
  (if (`self.IsCloseToAny?`)
    (goto _label)
    (else
      (`|SpawnActorFromClass` "/Game/Liam/BP/BP_Target.BP_Target_C" (`KismetMathLibrary.MakeTransform` (`self.newLocation`)) "Undefined" "MultiplyWithRoot" null null)
      (`KismetSystemLibrary.DelayUntilNextTick`)
      (`/Engine/EditorBlueprintResources/StandardMacros.FlipFlop`
        (:`A`
          (`/Engine/EditorBlueprintResources/StandardMacros.FlipFlop`
            (:`A`
              (set `self.previousLocation` _newlocation))
            (:`B`
              (set `self.previousLocation3` _newlocation))))
        (:`B`
          (set `self.previousLocation2` _newlocation))))))

(fn `UserConstructionScript`
  (`BoxComponent.SetBoxExtent` (`self.Box`) (`self.In Box Extent`) true))