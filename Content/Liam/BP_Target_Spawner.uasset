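; BP_Target_Spawner spawns BP_Target actors at random points inside a box volume.
; On BeginPlay it binds SpawnTarget to the first-person character's spawn dispatcher, then spawns an initial batch of three targets.
; Each later dispatch from the character adds another target at a new random point.
; The construction script sizes the box from the InBoxExtent variable, so each placed instance can define its own spawn area.
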(event `self.ReceiveBeginPlay`
  (bind _asbp_first_person_character (cast `/Game/FirstPerson/Blueprints/BP_FirstPersonCharacter` (`GameplayStatics.GetPlayerCharacter` 0)))
  (bind _output_get (set `self.As BP First Person Character` _asbp_first_person_character))
  (add `/Game/FirstPerson/Blueprints/BP_FirstPersonCharacter.SpawnDispatch` _output_get (delegate `Spawn Target`))
  (for _ (range 3)
    (`self.Spawn Target`)))

(event `Spawn Target`
  (bind _box (`self.Box`))
  (`|SpawnActorFromClass` "/Game/Liam/BP_Target.BP_Target_C" (`KismetMathLibrary.MakeTransform` (`KismetMathLibrary.RandomPointInBoundingBox` (`SceneComponent.K2_GetComponentLocation` _box) (`BoxComponent.GetScaledBoxExtent` _box))) "Undefined" "MultiplyWithRoot" null null))

(fn `UserConstructionScript`
  (`BoxComponent.SetBoxExtent` (`self.Box`) (`self.In Box Extent`) true))